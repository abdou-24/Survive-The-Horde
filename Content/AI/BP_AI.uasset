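; BP_AI is a zombie enemy character that detects, attacks and can be killed by the first-person player.
; Pawn sensing sets a "hasSeenPlayer?" Blackboard key on its AI controller.
; AttackPlayer uses a short forward sphere trace to play an attack montage and damage the player.
; HitEnemy subtracts Health, but its health check is unconnected, so any hit destroys the enemy and awards player score.
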(event `self.PawnSensing.OnSeePawn`
  (params (Pawn :type "Pawn Object Reference"))
  (cast `/Game/FirstPerson/Blueprints/BP_FirstPersonCharacter` Pawn)
  (`BlackboardComponent.SetValueAsBool` (`AIBlueprintHelperLibrary.GetBlackboard` (`AIBlueprintHelperLibrary.GetAIController` self)) "hasSeenPlayer?" true))

(event `Attack Player`
  (bind _returnvalue (`self.K2_GetActorLocation`))
  (bind (_outhit _returnvalue_2) (`KismetSystemLibrary.SphereTraceSingleForObjects` :`Start` _returnvalue :`End` (+ _returnvalue (* (`KismetMathLibrary.GetForwardVector` (`self.K2_GetActorRotation`)) 250.0)) :`Radius` 25.0 :`ObjectTypes` (`|MakeArray` "ObjectTypeQuery3" :!type "EObjectTypeQuery Enum") :`DrawDebugType` "ForDuration"))
  (if _returnvalue_2
    (bind (_bblockinghit _binitialoverlap _time _distance _location _impactpoint _normal _impactnormal _physmat _hitactor) (`GameplayStatics.BreakHitResult` _outhit))
    (cast `/Game/FirstPerson/Blueprints/BP_FirstPersonCharacter` _hitactor)
    (`self.PlayAnimMontage` "/Game/AI/Animation/Zombie_Attack_AnimMontage.Zombie_Attack_AnimMontage")
    (`GameplayStatics.ApplyDamage` _hitactor 5.0)))

(event `/Game/AI/EnemyDamage_Interface.Hit Enemy`
  (params (Damage :type "Float (double-precision)"))
  (bind _output_get (set `self.Health` (- (`self.Health`) Damage)))
  (if true
    (`KismetSystemLibrary.PrintString` "Enemy Killed" true true (struct :`R` 1.0 :`B` 0.046926 :`A` 1.0))
    (`self.K2_DestroyActor`)
    (bind _asbp_first_person_character (cast `/Game/FirstPerson/Blueprints/BP_FirstPersonCharacter` (`GameplayStatics.GetPlayerCharacter` 0)))
    (set `/Game/FirstPerson/Blueprints/BP_FirstPersonCharacter.Score` (+ (`/Game/FirstPerson/Blueprints/BP_FirstPersonCharacter.Score` _asbp_first_person_character) 5) _asbp_first_person_character)
    (else
      (`KismetSystemLibrary.PrintString` (`KismetStringLibrary.Conv_DoubleToString` _output_get) true true (struct :`R` 1.0 :`B` 0.046926 :`A` 1.0)))))

(fn `UserConstructionScript`)